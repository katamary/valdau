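; Base interactable that implements press-and-hold interaction, with an empty Action event as the hook for the result.
; Interact adds a loadbar widget and starts Held; Held and Released swap short named timers whose handlers step the push time up or down.
; Exceeding the push limit fires Action and calls RemoveLoadbar, as does releasing.
; RemoveLoadbar and UpdateWidget are empty stubs here, and neither timer is set to loop.
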(event `self.Interact`
  (bind _returnvalue (`|CreateWidget` "/Game/UI/Interactables/W_Interact_Loadbar.W_Interact_Loadbar_C" (`GameplayStatics.GetPlayerController` 0)))
  (bind _output_get (set `self.W_Interact_Loadbar_Ref` _returnvalue))
  (`UserWidget.AddToViewport` _output_get 0)
  (`self.Held`))

(event `Held`
  (`KismetSystemLibrary.K2_ClearAndInvalidateTimerHandle` (`self.ButtonReleaseTimer`))
  (bind _returnvalue (`KismetSystemLibrary.K2_SetTimer` null "HandleButtonHeldTimer" 0.01))
  (set `self.ButtonHeldTimer` _returnvalue))

(event `self.Released`
  (`KismetSystemLibrary.K2_ClearAndInvalidateTimerHandle` (`self.ButtonHeldTimer`))
  (bind _returnvalue (`KismetSystemLibrary.K2_SetTimer` null "HandleButtonReleaseTimer" 0.01))
  (set `self.ButtonReleaseTimer` _returnvalue)
  (`self.RemoveLoadbar`))

(event `self.Action`)

(fn `HandleButtonHeldTimer`
  (if (> (`self.ButonPushTime`) (`self.ButtonPushLimit`))
    (`self.Action`)
    (`KismetSystemLibrary.K2_ClearAndInvalidateTimerHandle` (`self.ButtonHeldTimer`))
    (`self.RemoveLoadbar`)
    (else
      (set `self.ButonPushTime` (+ (`self.ButonPushTime`) 0.01))
      (`self.UpdateWidget`))))

(fn `HandleButtonReleaseTimer`
  (bind _butonpushtime (`self.ButonPushTime`))
  (if (and (> (`self.ButtonPushLimit`) _butonpushtime) (> _butonpushtime 0.0))
    (set `self.ButonPushTime` (- (`self.ButonPushTime`) 0.01))
    (`self.UpdateWidget`)
    (else
      (`KismetSystemLibrary.K2_ClearAndInvalidateTimerHandle` (`self.ButtonHeldTimer`)))))

(fn `RemoveLoadbar`)

(fn `UpdateWidget`)

(fn `UserConstructionScript`)